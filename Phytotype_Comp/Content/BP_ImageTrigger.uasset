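; BP_ImageTrigger is an interactable trigger that shows an info panel with a title, text and image.
; Sphere overlap enables input and shows an interact prompt, and leaving removes the prompt and any open panel.
; Pressing E toggles between prompt and WBP_InfoPanel, switching cursor and input mode.
; A DoOnce adds the entry to the first-person character's AgendaSbloccata on first opening.
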(event `self.ReceiveActorBeginOverlap`
  (params (OtherActor :type "Actor Object Reference")))

(event `self.Sphere.OnComponentBeginOverlap`
  (params (OverlappedComponent :type "PrimitiveComponent Object Reference") (OtherActor :type "Actor Object Reference") (OtherComp :type "PrimitiveComponent Object Reference") (OtherBodyIndex :type Integer) (bFromSweep :type Boolean) (SweepResult :type "HitResult Structure (by ref)"))
  (set `self.Is Near Object` true)
  (`self.EnableInput` (`GameplayStatics.GetPlayerController` 0))
  (bind _returnvalue (`|CreateWidget` "/Game/Widget/WBP_InteractPrompt.WBP_InteractPrompt_C"))
  (bind _output_get (set `self.Interact Prompt Ref` _returnvalue))
  (`UserWidget.AddToViewport` _output_get 0))

(event `self.Sphere.OnComponentEndOverlap`
  (params (OverlappedComponent :type "PrimitiveComponent Object Reference") (OtherActor :type "Actor Object Reference") (OtherComp :type "PrimitiveComponent Object Reference") (OtherBodyIndex :type Integer))
  (`/Engine/EditorBlueprintResources/StandardMacros.IsValid` (`self.Interact Prompt Ref`)
    (:`Is Valid`
      (`Widget.RemoveFromParent` (`self.Interact Prompt Ref`))
      (set `self.Interact Prompt Ref` null)
      (set `self.Is Near Object` false)
      (`/Engine/EditorBlueprintResources/StandardMacros.IsValid` (`self.Current Widget`)
        (:`Is Valid`
          (`Widget.RemoveFromParent` (`self.Current Widget`))
          (set `self.Current Widget` null)
          (set `self.Widget Visible` false)
          (`self.DisableInput` (`GameplayStatics.GetPlayerController` 0))
          (set `PlayerController.bShowMouseCursor` false (`GameplayStatics.GetPlayerController` 0))
          (`WidgetBlueprintLibrary.SetInputMode_GameOnly` (`GameplayStatics.GetPlayerController` 0)))))))

(event `Key|E`
  (params (Key :type "Key Structure"))
  (:`Pressed`
    (if (`self.Is Near Object`)
      (if (`self.Widget Visible`)
        (`/Engine/EditorBlueprintResources/StandardMacros.IsValid` (`self.Current Widget`)
          (:`Is Valid`
            (`Widget.RemoveFromParent` (`self.Current Widget`))
            (set `self.Current Widget` null)
            (set `self.Widget Visible` false)
            (set `PlayerController.bShowMouseCursor` false (`GameplayStatics.GetPlayerController` 0))
            (`WidgetBlueprintLibrary.SetInputMode_GameOnly` (`GameplayStatics.GetPlayerController` 0))
            (bind _returnvalue (`|CreateWidget` "/Game/Widget/WBP_InteractPrompt.WBP_InteractPrompt_C"))
            (bind _output_get (set `self.Interact Prompt Ref` _returnvalue))
            (`UserWidget.AddToViewport` _output_get 0))
          (:`Is Not Valid`
            (set `self.Widget Visible` false)))
        (else
          (`/Engine/EditorBlueprintResources/StandardMacros.IsValid` (`self.Interact Prompt Ref`)
            (:`Is Valid`
              (`Widget.RemoveFromParent` (`self.Interact Prompt Ref`))
              (`|ExecutionSequence`
                (:`then_0`
                  (bind _returnvalue_2 (`|CreateWidget` "/Game/Widget/WBP_InfoPanel.WBP_InfoPanel_C" null (`self.Displayed Text`) (`self.Image To Show`) (`self.Displayed Title`)))
                  (bind _output_get_2 (set `self.Current Widget` _returnvalue_2))
                  (`UserWidget.AddToViewport` _output_get_2 0)
                  (set `PlayerController.bShowMouseCursor` true (`GameplayStatics.GetPlayerController` 0))
                  (`WidgetBlueprintLibrary.SetInputMode_GameAndUIEx` (`GameplayStatics.GetPlayerController` 0) (`self.Current Widget`))
                  (set `self.Widget Visible` true))
                (:`then_1`
                  (`/Engine/EditorBlueprintResources/StandardMacros.DoOnce` false
                    (:`Completed`
                      (bind _asbp_first_person_character (cast `/Game/FirstPerson/Blueprints/BP_FirstPersonCharacter` (`GameplayStatics.GetPlayerCharacter` 0)))
                      (`KismetArrayLibrary.Array_Add` (`/Game/FirstPerson/Blueprints/BP_FirstPersonCharacter.AgendaSbloccata` _asbp_first_person_character) (make `/Game/Widget/F_PaginaAgenda` (`self.Displayed Text`) (`self.Image To Show`) (`self.Displayed Title`))))))))))))))

(fn `UserConstructionScript`)