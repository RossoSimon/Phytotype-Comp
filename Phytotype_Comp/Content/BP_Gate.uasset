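; BP_Gate is a level exit that opens the next level once the first-person character overlaps its trigger with all banners collected.
; On success it plays a fog-gate sound, disables input, fades to white and copies the character's unlocked agenda state into GI_Partita before loading the level by name.
; Otherwise it shows a WBP_GateMessaggio widget, using a DoOnce reset after a delay to prevent repeated messages.
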(event `self.Trigger.OnComponentBeginOverlap`
  (params (OverlappedComponent :type "PrimitiveComponent Object Reference") (OtherActor :type "Actor Object Reference") (OtherComp :type "PrimitiveComponent Object Reference") (OtherBodyIndex :type Integer) (bFromSweep :type Boolean) (SweepResult :type "HitResult Structure (by ref)"))
  (bind _returnvalue (`GameplayStatics.GetPlayerController` 0))
  (bind _asbp_first_person_character (cast `/Game/FirstPerson/Blueprints/BP_FirstPersonCharacter` OtherActor))
  (if (== (`/Game/FirstPerson/Blueprints/BP_FirstPersonCharacter.BannersRaccolti` _asbp_first_person_character) (`/Game/FirstPerson/Blueprints/BP_FirstPersonCharacter.BannersTotali` _asbp_first_person_character))
    (`GameplayStatics.PlaySound2D` "/Game/Dark_Souls_-_New_Area_Fog_Gate_Sound_Effect.Dark_Souls_-_New_Area_Fog_Gate_Sound_Effect" 1.0 1.0 0.0 null null)
    (`self.DisableInput` _returnvalue _returnvalue)
    (`PlayerCameraManager.StartCameraFade` (`GameplayStatics.GetPlayerCameraManager` 0) 0.0 1.0 3.0 (struct :`R` 1.0 :`G` 1.0 :`B` 1.0 :`A` 1.0) false true)
    (`KismetSystemLibrary.Delay` 3.1)
    (bind _asbp_first_person_character_2 (cast `/Game/FirstPerson/Blueprints/BP_FirstPersonCharacter` (`GameplayStatics.GetPlayerCharacter` 0)))
    (bind _asgi_partita (cast `/Game/GI_Partita` (`GameplayStatics.GetGameInstance`)))
    (set `/Game/GI_Partita.AgendaDISalvataggio` (`/Game/FirstPerson/Blueprints/BP_FirstPersonCharacter.AgendaSbloccata` _asbp_first_person_character_2) _asgi_partita)
    (`GameplayStatics.OpenLevel` (`self.NomeProssimoLivello`))
    (else
      (`/Engine/EditorBlueprintResources/StandardMacros.DoOnce` false :!label _label
        (:`Completed`
          (bind _returnvalue_2 (`|CreateWidget` "/Game/Widget/WBP_GateMessaggio.WBP_GateMessaggio_C"))
          (`UserWidget.AddToViewport` _returnvalue_2 0)
          (`KismetSystemLibrary.Delay` 3.5)
          (goto _label :!via `Reset`))))))

(fn `UserConstructionScript`)